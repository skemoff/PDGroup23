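; DynamicPlatformRock is a configurable moving platform that travels toward an end location while a PHBlueprint actor overlaps its trigger Box.
; The construction script applies mesh, scale and rotation to MainPlatform and EndPlatformReference, placing the latter at EndLocation to mark the destination.
; Overlap plays the MovePlatform timeline, with play rate derived from Duration, lerping MainPlatform's relative location from its starting point.
; Leaving the Box reverses the timeline, returning the platform toward its start.
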(event `self.ReceiveBeginPlay`
  (set `self.Start Location` (`SceneComponent.RelativeLocation` (`self.MainPlatform`))))

(event `self.Box.OnComponentBeginOverlap`
  (params (OverlappedComponent :type "PrimitiveComponent Object Reference") (OtherActor :type "Actor Object Reference") (OtherComp :type "PrimitiveComponent Object Reference") (OtherBodyIndex :type Integer) (bFromSweep :type Boolean) (SweepResult :type "HitResult Structure (by ref)"))
  (cast `/Game/Blueprints/PHBlueprint` OtherActor)
  (`TimelineComponent.SetPlayRate` (`self.Move Platform`) (/ 1.0 (`self.Duration`)))
  (bind (_direction _move_track) (`Timeline|Move Platform` :!label _label)
    (:`Update`
      (`SceneComponent.K2_SetRelativeLocation` (`self.MainPlatform`) (`KismetMathLibrary.VLerp` (`self.Start Location`) (`self.End Location`) _move_track) false false))))

(event `self.Box.OnComponentEndOverlap`
  (params (OverlappedComponent :type "PrimitiveComponent Object Reference") (OtherActor :type "Actor Object Reference") (OtherComp :type "PrimitiveComponent Object Reference") (OtherBodyIndex :type Integer))
  (cast `/Game/Blueprints/PHBlueprint` OtherActor)
  (`TimelineComponent.SetPlayRate` (`self.Move Platform`) (/ 1.0 (`self.Duration`)))
  (goto _label :!via `Reverse`))

(fn `UserConstructionScript`
  (bind _mainplatform (`self.MainPlatform`))
  (bind _end_platform_reference (`self.End Platform Reference`))
  (bind _platform_mesh (`self.Platform Mesh`))
  (`StaticMeshComponent.SetStaticMesh` _mainplatform _platform_mesh)
  (`StaticMeshComponent.SetStaticMesh` _end_platform_reference _platform_mesh)
  (`SceneComponent.SetRelativeScale3D` _mainplatform (`self.Scale`))
  (`SceneComponent.SetRelativeScale3D` _end_platform_reference (`self.Scale`))
  (`SceneComponent.K2_SetRelativeRotation` _mainplatform (`self.Rotation`) false false)
  (`SceneComponent.K2_SetRelativeRotation` _end_platform_reference (`self.Rotation`) false false)
  (`SceneComponent.K2_SetRelativeLocation` _end_platform_reference (`self.End Location`) false false))