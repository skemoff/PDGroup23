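; Frog boss enemy with flipbook sprite animation that wanders, chases the player and deals contact damage.
; PawnSensing starts an AI move toward a seen PHBlueprint, and a retriggerable delay clears the sighting flag, returning Tick to delayed random wandering.
; Box overlaps damage other actors; incoming damage lowers HP, destroying the frog at zero.
; Health text updates only during sightings, while UpdateAnimation picks idle or jump flipbooks from movement.
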(event `self.ReceiveTick`
  (params (DeltaSeconds :type "Float (single-precision)"))
  (if (not (`self.CanSeeEnemy?`))
    (`KismetSystemLibrary.Delay` 1.0)
    (`|AIMoveTo` self (`NavigationSystemV1.K2_GetRandomReachablePointInRadius` (`self.K2_GetActorLocation`) 100.0 null null) null)
    (else
      (`TextRenderComponent.K2_SetText` (`self.Health`) (`KismetTextLibrary.Conv_IntToText` (`KismetMathLibrary.FTrunc` (`self.HP`))))
      (if (<= (`self.HP`) 0.0)
        (`self.K2_DestroyActor`)))))

(event `self.Box.OnComponentBeginOverlap`
  (params (OverlappedComponent :type "PrimitiveComponent Object Reference") (OtherActor :type "Actor Object Reference") (OtherComp :type "PrimitiveComponent Object Reference") (OtherBodyIndex :type Integer) (bFromSweep :type Boolean) (SweepResult :type "HitResult Structure (by ref)"))
  ;[1 1 1] ENEMY DAMAGING FUNCTION
  (if (!= OtherActor self)
    (`GameplayStatics.ApplyDamage` OtherActor 34.0 null self)))

(event `self.ReceiveAnyDamage`
  (params (Damage :type "Float (single-precision)") (DamageType :type "DamageType Object Reference") (InstigatedBy :type "Controller Object Reference") (DamageCauser :type "Actor Object Reference"))
  (set `self.HP` (- (`self.HP`) Damage))
  (if (<= (`self.HP`) 0.0)
    (`self.K2_DestroyActor`)))

(event `UpdateAnimation`
  (bind (_returnvalue_x _returnvalue_y _returnvalue_z) (`KismetMathLibrary.BreakVector` (`self.GetVelocity`)))
  ;[1 1 1] Animation Handler
  (if (`NavMovementComponent.IsFalling` (`self.CharacterMovement`))
    (`PaperFlipbookComponent.SetFlipbook` (`self.Frog Sprite`) (select `bool` (< _returnvalue_z 0.0) :`false` "/Game/Sprites/PlaceHolder/frog/jump/frog-jump-FB.frog-jump-FB" :`true` "/Game/Sprites/PlaceHolder/frog/jump/frog-jump-FB.frog-jump-FB" :!type "PaperFlipbook Object Reference"))
    (else
      (`PaperFlipbookComponent.SetFlipbook` (`self.Frog Sprite`) (select `bool` (> (`KismetMathLibrary.VSize` (`MovementComponent.Velocity` (`self.CharacterMovement`))) 0.0) :`false` "/Game/Sprites/PlaceHolder/frog/idle/frog-idle-FB.frog-idle-FB" :`true` "/Game/Sprites/PlaceHolder/frog/jump/frog-jump-FB.frog-jump-FB" :!type "PaperFlipbook Object Reference")))))

(event `self.PawnSensing.OnSeePawn`
  (params (Pawn :type "Pawn Object Reference"))
  ;[1 1 1] Enemy chases player
  (bind _asphblueprint (cast `/Game/Blueprints/PHBlueprint` Pawn))
  (`|ExecutionSequence`
    (:`then_0`
      (set `self.CanSeeEnemy?` true)
      (`|AIMoveTo` self (0.0 0.0 0.0) _asphblueprint))
    (:`then_1`
      (`KismetSystemLibrary.RetriggerableDelay` 0.5)
      (set `self.CanSeeEnemy?` false))))

(fn `UserConstructionScript`)